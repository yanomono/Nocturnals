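; Player controller that handles pause, sight switching, dialogue advancing and clicking on symptoms.
; Escape flip-flops between creating a pause widget with the game paused and removing it to resume.
; DialogueMode gates input: when on, NextDialogue advances DialogueRef; when off, SwitchSight toggles CameraRef between normal and supernatural views.
; Outside dialogue, left click traces under the cursor for BP_Symptom actors, currently only printing a debug string on a hit.
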(event EventBeginPlay
  (Variables|Default|SetGameInstanceRef (Game|GetGameInstance)))

(event Input|ActionEvents|InputActionSwitchSight
  (params (Key :type Key%20Structure :default "None"))
  (bind _cameraref (Variables|Default|GetCameraRef))
  (:Pressed
    (if (not (Variables|Default|GetDialogueMode))
      (Utilities|FlowControl|FlipFlop
        (:A
          (Development|PrintString "supernatural")
          (Default|SupernaturalViewMode _cameraref))
        (:B
          (Development|PrintString "normal")
          (Default|NormalViewMode _cameraref))))))

(event Input|ActionEvents|InputActionNextDialogue
  (params (Key :type Key%20Structure :default "None"))
  (:Pressed
    (if (Variables|Default|GetDialogueMode)
      (bind _dialogueref (Variables|Default|GetDialogueRef)
        (:then
          (Class|BPIntDialogueInputs|NextDialogue(Message) _dialogueref))
        (:else)))))

(event Input|ActionEvents|InputActionLMB
  (params (Key :type Key%20Structure :default "None"))
  (bind _array (Utilities|Array|MakeArray "ObjectTypeQuery7"))
  (bind (_hitresult _returnvalue) (Class|PlayerController|GetHitResultUnderCursorforObjects _array true))
  (:Pressed
    (if (not (Variables|Default|GetDialogueMode))
      (if _returnvalue
        (Utilities|Casting|CastToBP_Symptom (.HitActor (Collision|BreakHitResult _hitresult)))
        (Development|PrintString "symptom")))))

(event Input|KeyboardEvents|Escape
  (params (Key :type Key%20Structure :default "None"))
  (:Pressed
    (Utilities|FlowControl|FlipFlop
      (:A
        (bind _returnvalue (UserInterface|CreateWidget "/Game/UI/WBP_PauseMenu.WBP_PauseMenu_C"))
        (UserInterface|Viewport|AddtoViewport _returnvalue 0)
        (Game|SetGamePaused true))
      (:B
        (Widget|RemovefromParent _returnvalue)
        (Game|SetGamePaused false)))))

(fn ConstructionScript)