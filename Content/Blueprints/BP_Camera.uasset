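; Player camera actor that becomes the view target on BeginPlay, registers itself with PC_Player, and handles normal and supernatural view modes.
; The two view-mode events replace the camera's post-process settings, switching between a white and a red-orange color.
; Eyelids plays a timeline forward or backward to slide two mirrored Paper sprites like eyelids.
; An event track on that timeline rotates the Scene component 90 degrees for supernatural view, or back to zero.
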(event Custom|SupernaturalViewMode
  (Variables|/Script/Engine.CameraComponent|SetPostProcessSettings (Variables|Default|GetCamera) (Utilities|Struct|MakePostProcessSettings "(R=1.000000,G=0.122801,B=0.000000,A=1.000000)")))

(event Custom|NormalViewMode
  (Variables|/Script/Engine.CameraComponent|SetPostProcessSettings (Variables|Default|GetCamera) (Utilities|Struct|MakePostProcessSettings "(R=1.000000,G=1.000000,B=1.000000,A=1.000000)")))

(event Custom|Eyelids
  (params (Supernat? :type Boolean))
  (bind _scene (Variables|Default|GetScene))
  (if Supernat?
    (bind (_direction _newtrack_0) (Timeline|Timeline_0 PlayFromStart)
      (:Update
        (Transformation|SetRelativeLocation (Variables|Default|GetPaperSprite) (Math|Vector|MakeVector 1.5e+02 0.0 (Math|Float|Lerp 2e+03 7.7e+02 _newtrack_0)) false false)
        (Transformation|SetRelativeLocation (Variables|Default|GetPaperSprite1) (Math|Vector|MakeVector 1.5e+02 0.0 (* (Math|Float|Lerp 2e+03 7.7e+02 _newtrack_0) -1.0)) false false))
      (:NewTrack_1
        (if Supernat?
          (Transformation|SetRelativeRotation _scene "0, 0,90.000000" false false)
          (else
            (Transformation|SetRelativeRotation _scene "0, 0, 0" false false)))))
    (else
      (Timeline|Timeline_0 ReverseFromEnd))))

(event EventBeginPlay
  (bind _returnvalue (Game|GetPlayerController 0))
  (Game|Player|SetViewTargetwithBlend _returnvalue self 0.0 "VTBlend_Linear" 0.0 false)
  (bind _aspc_player (Utilities|Casting|CastToPC_Player _returnvalue))
  (Variables|/Game/Blueprints/PC_Player.PC_Player_C|SetCameraRef _aspc_player self))

(fn ConstructionScript)