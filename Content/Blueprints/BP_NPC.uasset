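; Patient NPC that slides in to a dialogue spot, talks, and slides out once completed, advancing its manager to the next character.
; SelectDialogue prefers unread, flag-eligible priority tables, then default ones, falling back to the last eligible read table, for display in WBP_Dialogue.
; Closing dialogue can reveal the player HUD, and emotions swap the Paper2D sprite.
; The construction script spawns BP_Symptom child actors with radius, supernatural state and flags from SymptomsToSpawn.
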(event Custom|CustomerCompleted
  (params (Success? :type Boolean))
  (Variables|Default|SetCompleted true)
  (if Success?
    (Development|PrintString "success")
    (else
      (Development|PrintString "failure"))))

(event Custom|OpenDialogue
  (bind _dialogue (CallFunction|SelectDialogue))
  (Utilities|IsValid _dialogue
    (:Is%20Valid
      (bind _output_get (Variables|Default|SetDialogueForDisplay _dialogue))
      (bind _returnvalue (UserInterface|CreateWidget "/Game/UI/DialogueUI/WBP_Dialogue.WBP_Dialogue_C" 0 _output_get self))
      (UserInterface|Viewport|AddtoViewport _returnvalue 0))))

(event Custom|Emote
  (params (Emotion :type Enum_Emotions%20Enum :default "NewEnumerator0"))
  (Rendering|Components|Sprite|SetSprite (Variables|Default|GetPaperSprite) (.Value (Utilities|Map|Find (Variables|Default|GetEmotionSprites) Emotion))))

(event Custom|SlideCharacter
  (params (StartVector :type Vector) (EndVector :type Vector))
  (bind _newtrack_0 (Timeline|Timeline_0 PlayFromStart)
    (:Update
      (Transformation|SetActorLocation (Math|Vector|Lerp(Vector) StartVector EndVector _newtrack_0) false false))))

(event Custom|ActivateCharacter
  (CallFunction|SlideCharacter (Transformation|GetActorLocation (Variables|Default|GetEntryPoint)) (Transformation|GetActorLocation (Variables|Default|GetDialogueSpot)))
  (Utilities|FlowControl|Delay (Variables|Default|GetPatientSlideDelay))
  (CallFunction|OpenDialogue))

(event Custom|Incorrect
  (Default|Incorrect (Variables|Default|GetManagerRef)))

(event EventBeginPlay
  (bind _asbp_game_instnace (Utilities|Casting|CastToBP_GameInstnace (Game|GetGameInstance)))
  (bind _output_get (Variables|Default|SetGameInstanceRef _asbp_game_instnace))
  (Variables|/Game/Blueprints/BP_GameInstnace.BP_GameInstnace_C|SetNPCRef _output_get self)
  (Transformation|SetActorLocation (Transformation|GetActorLocation (Variables|Default|GetEntryPoint)) false false)
  (Rendering|Components|Sprite|SetSprite (Variables|Default|GetPaperSprite) (.Value (Utilities|Map|Find (Variables|Default|GetEmotionSprites) (Utilities|Enum|LiteralenumEnum_Emotions "NewEnumerator0")))))

(event EventDialogueClosed
  (bind _managerref (Variables|Default|GetManagerRef))
  (if (Variables|Default|GetTools)
    (bind _aspc_player (Utilities|Casting|CastToPC_Player (Game|GetPlayerController 0)))
    (Default|ShowHUD _aspc_player)
    (Variables|Default|SetTools false))
  (if (Variables|Default|GetCompleted)
    (CallFunction|SlideCharacter (Transformation|GetActorLocation (Variables|Default|GetDialogueSpot)) (Transformation|GetActorLocation (Variables|Default|GetExitPoint)))
    (Utilities|FlowControl|Delay 1.0)
    (Variables|/Game/Blueprints/BP_CharacterManager.BP_CharacterManager_C|SetCurrentIndex _managerref (+ (Variables|/Game/Blueprints/BP_CharacterManager.BP_CharacterManager_C|GetCurrentIndex _managerref) 1))
    (Default|NextCharacter _managerref)))

(fn ConstructionScript
  (bind _symptomstospawn (Variables|Default|GetSymptomsToSpawn))
  (for _index (range 0 (Utilities|Array|LastIndex _symptomstospawn))
    (bind _returnvalue (AddComponent|AddChildActorComponent false (Math|Transform|MakeTransform (Math|Vector|MakeVector (.X (Math|Vector|BreakVector (.position (Utilities|Array|Get(acopy) _symptomstospawn _index)))) 3.0 (.Z (Math|Vector|BreakVector (.position (Utilities|Array|Get(acopy) _symptomstospawn _index))))))))
    (ChildActorComponent|SetChildActorClass _returnvalue "/Game/Blueprints/BP_Symptom.BP_Symptom_C")
    (bind _asbp_symptom (Utilities|Casting|CastToBP_Symptom (Variables|/Script/Engine.ChildActorComponent|GetChildActor _returnvalue)))
    (Components|Sphere|SetSphereRadius (Variables|/Game/Blueprints/BP_Symptom.BP_Symptom_C|GetSphere _asbp_symptom) (.radius (Utilities|Array|Get(acopy) _symptomstospawn _index)) true)
    (Variables|/Game/Blueprints/BP_Symptom.BP_Symptom_C|SetSupernatural? _asbp_symptom (.supernatural? (Utilities|Array|Get(acopy) _symptomstospawn _index)))
    (for _array_element (.giveflags (Utilities|Array|Get(acopy) _symptomstospawn _index))
      (Utilities|Array|AddUnique (Variables|/Game/Blueprints/BP_Symptom.BP_Symptom_C|GetGiveFlags _asbp_symptom) _array_element))))

(fn SelectDialogue
  (bind _gameinstanceref (Variables|Default|GetGameInstanceRef))
  (bind _gameinstanceref_2 (Variables|Default|GetGameInstanceRef))
  ;[1 1 1] Check priority dialogues first, pick first dialgoue that meets the conditions and hasn't been read yet
  (bind _array_element (Utilities|Array|ForEachLoopwithBreak (Variables|Default|GetPriorityDialogueList) :!label _label)
    (:LoopBody
      (bind _read_ (Default|CheckReadTableStatus _gameinstanceref_2 (.DataTable (Utilities|Struct|BreakStruct_DataTableSelection _array_element))))
      (if (not _read_) ; has it been read yet? skip already read ones
        (if (== (Utilities|Array|Length (.RequiredFlag (Utilities|Struct|BreakStruct_DataTableSelection _array_element))) 0) ; does it require no flags?
          (LocalVariables|SetDialogueToDisplay (.DataTable (Utilities|Struct|BreakStruct_DataTableSelection _array_element)) :!label _label_2)
          (goto _label Break)
          (else
            (bind _checkresult (Default|MultiFlagCheck _gameinstanceref_2 (.RequiredFlag (Utilities|Struct|BreakStruct_DataTableSelection _array_element)) (.SelectionLogic (Utilities|Struct|BreakStruct_DataTableSelection _array_element))))
            (if _checkresult ; were the conditions met?
              (goto _label_2))))))
    (:Completed
      (bind _dialoguetodisplay (LocalVariables|GetDialogueToDisplay)
        (:then
          (return _dialoguetodisplay) ; stop here and return the result if a dialogue was found
        )
        (:else
          ;[1 1 1] If there's no new priority dialogue to display, pick a default dialogue - first unread that meets conditions or last read if there's no valid new dialogue
          (bind _array_element_2 (Utilities|Array|ForEachLoopwithBreak (Variables|Default|GetDefaultDialogueList) :!label _label_3)
            (:LoopBody
              (if (== (Utilities|Array|Length (.RequiredFlag (Utilities|Struct|BreakStruct_DataTableSelection _array_element_2))) 0) ; does it require no flags?
                (bind _output_get (LocalVariables|SetDialogueToDisplay (.DataTable (Utilities|Struct|BreakStruct_DataTableSelection _array_element_2)) :!label _label_4))
                (bind _read__2 (Default|CheckReadTableStatus _gameinstanceref _output_get))
                (if (not _read__2) ; break if it's a new unread dialogue
                  (goto _label_3 Break))
                (else
                  (bind _checkresult_2 (Default|MultiFlagCheck _gameinstanceref (.RequiredFlag (Utilities|Struct|BreakStruct_DataTableSelection _array_element_2)) (.SelectionLogic (Utilities|Struct|BreakStruct_DataTableSelection _array_element_2))))
                  (if _checkresult_2 ; were the conditions met?
                    (goto _label_4)))))
            (:Completed
              (return (LocalVariables|GetDialogueToDisplay)) ; if no dialogue was found, the widget won't be created
            )))))))