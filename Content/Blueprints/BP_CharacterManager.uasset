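; BP_CharacterManager activates a character from its list and tracks wrong attempts against it.
; On BeginPlay it hands itself to PC_Player and every listed character, then calls NextCharacter.
; NextCharacter clears the attempt count and activates the character at the current index, without advancing that index.
; SpiritSprite picks one of two emotes for the current character based on a Supernatural flag, while Incorrect increments the attempt count.
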(event Custom|NextCharacter
  (Variables|Default|SetAttempts 0)
  (bind _output_get (Variables|Default|SetCurrentCharacter (Utilities|Array|Get(acopy) (Variables|Default|GetCharacters) (Variables|Default|GetCurrentIndex))))
  (Default|ActivateCharacter _output_get))

(event Custom|SpiritSprite
  (params (Supernatural? :type Boolean))
  (bind _currentcharacter (Variables|Default|GetCurrentCharacter))
  (if Supernatural?
    (Default|Emote _currentcharacter "NewEnumerator2")
    (else
      (Default|Emote _currentcharacter "NewEnumerator0"))))

(event Custom|Incorrect
  (Variables|Default|SetAttempts (+ (Variables|Default|GetAttempts) 1)))

(event EventBeginPlay
  (bind _aspc_player (Utilities|Casting|CastToPC_Player (Game|GetPlayerController 0)))
  (bind _output_get (Variables|Default|SetPlayerRef _aspc_player))
  (Variables|/Game/Blueprints/PC_Player.PC_Player_C|SetManagerRef _output_get self)
  (for _array_element (Variables|Default|GetCharacters)
    (Variables|/Game/Blueprints/BP_NPC.BP_NPC_C|SetManagerRef _array_element self))
  (CallFunction|NextCharacter))

(fn ConstructionScript)