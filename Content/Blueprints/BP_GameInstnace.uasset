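; Game instance that holds story flags and read-dialogue state, with functions to update and query them.
; Flag checks support a {NOT} prefix per flag and AND/OR/NOT logic across lists.
; Read status is tracked per DataTable, by object name, and per row, creating missing entries on lookup.
; ClearSaveData wipes both stores and resets apples, the NPC animation and player walk speed.
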(fn AddFlag
  (params (NewFlag :type String))
  (Utilities|Array|AddUnique (Variables|Default|GetGatheredFlags) NewFlag))

(fn RemoveFlag
  (params (Flag :type String%20%28by%20ref%29))
  (Utilities|Array|RemoveItem (Variables|Default|GetGatheredFlags) Flag))

(fn SaveReadDialogueTable
  (params (DataTable :type Data%20Table%20Object%20Reference) (Item%20Read? :type Boolean))
  (bind _readdialoguesave (Variables|Default|GetReadDialogueSave))
  (bind (_read_ _saveindex) (CallFunction|CheckReadTableStatus DataTable)) ; where in the save array is it?
  (if (not (Math|Boolean|Equal(Boolean) _read_ Item%20Read?)) ; don't do anything if the status doesn't change
    (Utilities|Array|SetArrayElem _readdialoguesave _saveindex (Utilities|Struct|MakeStruct_ReadDialogue (.SaveName (Utilities|Struct|BreakStruct_ReadDialogue (Utilities|Array|Get(acopy) _readdialoguesave _saveindex))) Item%20Read? (.ReadLineList (Utilities|Struct|BreakStruct_ReadDialogue (Utilities|Array|Get(acopy) _readdialoguesave _saveindex)))))))

(fn SaveReadDialogueLine
  (params (DataTable :type Data%20Table%20Object%20Reference) (RowName :type Name%20%28by%20ref%29) (Read? :type Boolean%20%28by%20ref%29))
  (bind _saveindex (CallFunction|CheckReadTableStatus DataTable))
  (Utilities|Map|Add (.ReadLineList (Utilities|Struct|BreakStruct_ReadDialogue (Utilities|Array|Get(acopy) (Variables|Default|GetReadDialogueSave) _saveindex))) RowName Read?) ; adding a key that has the same name as one already in the map overrides it
)

(fn CheckReadTableStatus
  (params (DataTable :type Data%20Table%20Object%20Reference))
  (bind _returnvalue (Utilities|GetObjectName DataTable))
  (bind _tempboolmap (LocalVariables|GetTempBoolMap))
  ;[1 1 1] Check if you already saved this name
  (bind (_array_element _array_index) (Utilities|Array|ForEachLoopwithBreak (Variables|Default|GetReadDialogueSave) :!label _label)
    (:LoopBody
      (if (Utilities|Enum|Equal(Enum) (.SaveName (Utilities|Struct|BreakStruct_ReadDialogue _array_element)) _returnvalue)
        (LocalVariables|SetTableFound true)
        (LocalVariables|SetRead (.ReadTable? (Utilities|Struct|BreakStruct_ReadDialogue _array_element)))
        (LocalVariables|SetIndex _array_index)
        (goto _label Break)))
    (:Completed
      (if (LocalVariables|GetTableFound)
        (return (LocalVariables|GetRead) (LocalVariables|GetIndex))
        (else
          ;[1 1 1] Create a new entry if nothing was found
          (bind _outrownames (DataTable|GetDataTableRowNames DataTable))
          (for _array_element_2 _outrownames
            (Utilities|Map|Add _tempboolmap _array_element_2 false) ; fill a temporary map with all row names and attached booleans
          )
          (bind _returnvalue_2 (Utilities|Array|Add (Variables|Default|GetReadDialogueSave) (Utilities|Struct|MakeStruct_ReadDialogue _returnvalue false _tempboolmap))) ; when done make the map pernament in the saved array
          (return false _returnvalue_2))))))

(fn CheckReadLineStatus
  (params (DataTable :type Data%20Table%20Object%20Reference) (RowName :type Name%20%28by%20ref%29))
  (bind _saveindex (CallFunction|CheckReadTableStatus DataTable)) ; which table is it?
  (if (.ReturnValue (Utilities|Map|Find (.ReadLineList (Utilities|Struct|BreakStruct_ReadDialogue (Utilities|Array|Get(acopy) (Variables|Default|GetReadDialogueSave) _saveindex))) RowName)) ; was the row found?
    (return (.Value (Utilities|Map|Find (.ReadLineList (Utilities|Struct|BreakStruct_ReadDialogue (Utilities|Array|Get(acopy) (Variables|Default|GetReadDialogueSave) _saveindex))) RowName))) ; if yes, return the read/not read bool
    (else
      (Utilities|Map|Add (.ReadLineList (Utilities|Struct|BreakStruct_ReadDialogue (Utilities|Array|Get(acopy) (Variables|Default|GetReadDialogueSave) _saveindex))) RowName false) ; add a new entry in case it was missed during setup or new lines were added in an update
      (return false))))

(fn SingleFlagCheck
  (params (RequiredFlag :type String))
  (bind _returnvalue (Utilities|String|Contains RequiredFlag "{NOT}" true))
  (bind _array_element (Utilities|Array|ForEachLoopwithBreak (Variables|Default|GetGatheredFlags) :!label _label)
    (:LoopBody
      (if (Utilities|Enum|Equal(Enum) _array_element (Utilities|String|SelectString (Utilities|String|RightChop RequiredFlag 5) RequiredFlag _returnvalue))
        (LocalVariables|SetCheckOutcome true)
        (goto _label Break)))
    (:Completed
      (return (select _returnvalue (not (LocalVariables|GetCheckOutcome)) (LocalVariables|GetCheckOutcome))))))

(fn MultiFlagCheck
  (params (RequiredFlags :type Array%20of%20Strings) (SelectionLogic :type Enum_LogicStates%20Enum :default "NewEnumerator0"))
  (switch Utilities|FlowControl|Switch|SwitchonEnum_LogicStates SelectionLogic
    (:NewEnumerator0
      (bind _array_element (Utilities|Array|ForEachLoopwithBreak RequiredFlags :!label _label)
        (:LoopBody
          (bind _checkresult (CallFunction|SingleFlagCheck _array_element))
          (if _checkresult
            (LocalVariables|SetCheckOutcome true)
            (else
              (LocalVariables|SetCheckOutcome false)
              (goto _label Break))))
        (:Completed
          (return (LocalVariables|GetCheckOutcome)))))
    (:NewEnumerator1
      (bind _array_element_2 (Utilities|Array|ForEachLoopwithBreak RequiredFlags :!label _label_2)
        (:LoopBody
          (bind _checkresult_2 (CallFunction|SingleFlagCheck _array_element_2))
          (if _checkresult_2
            (LocalVariables|SetCheckOutcome true)
            (goto _label_2 Break)))
        (:Completed
          (return (LocalVariables|GetCheckOutcome)))))
    (:NewEnumerator2
      (bind _array_element_3 (Utilities|Array|ForEachLoopwithBreak RequiredFlags :!label _label_3)
        (:LoopBody
          (bind _checkresult_3 (CallFunction|SingleFlagCheck _array_element_3))
          (if _checkresult_3
            (LocalVariables|SetCheckOutcome true)
            (goto _label_3 Break)))
        (:Completed
          (return (not (LocalVariables|GetCheckOutcome))))))))

(fn ClearSaveData
  (Utilities|Array|Clear (Variables|Default|GetGatheredFlags))
  (Utilities|Array|Clear (Variables|Default|GetReadDialogueSave))
  (Default|ResetApples (Variables|Default|GetAppleManagerRef))
  (Variables|Default|SetApplesCollected 0)
  (Default|PlayAnimation (Variables|Default|GetNPCRef) "Reset")
  (bind _asbp_player (Utilities|Casting|CastToBP_Player (Game|Player|GetPlayerPawn 0)))
  (Default|ChangeWalkSpeed _asbp_player "600"))